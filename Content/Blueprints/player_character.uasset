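; Paper2D side-scroller player character with movement along X, jumping, wall sliding, wall jumping and a short attack.
; Tick picks the flipbook from slide and velocity state, flips control yaw by X direction and runs the wall check.
; While falling, a short forward trace detects walls and turns the character along the hit normal, so a wall jump launches forward and up.
; Attacking briefly locks the attack flipbook through a delayed flag.
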(event `Wallslide`
  (bind _returnvalue (`self.K2_GetActorLocation`))
  (bind _charactermovement (`self.CharacterMovement`))
  (if (< (.z (`MovementComponent.Velocity` (`self.CharacterMovement`))) 0.0)
    (bind (_outhit _returnvalue_2) (`KismetSystemLibrary.LineTraceSingle` _returnvalue (+ _returnvalue (* (`self.GetActorForwardVector`) 10.0)) "TraceTypeQuery1"))
    (if _returnvalue_2
      (set `self.Wallsliding` true)
      (bind (_returnvalue_roll _returnvalue_pitch _returnvalue_yaw) (`KismetMathLibrary.BreakRotator` (`KismetMathLibrary.Conv_VectorToRotator` (`.ImpactNormal` (`GameplayStatics.BreakHitResult` _outhit)))))
      (`self.K2_SetActorRotation` (`KismetMathLibrary.MakeRotator` 0.0 0.0 (+ 0.0 _returnvalue_yaw)))
      (set `MovementComponent.Velocity` (`KismetMathLibrary.VInterpTo` (0.0 0.0 0.0) (`MovementComponent.Velocity` _charactermovement) (`GameplayStatics.GetWorldDeltaSeconds`) 100.0) _charactermovement)
      (else
        (set `self.Wallsliding` false)))
    (else
      (set `self.Wallsliding` false))))

(event `InputAction|jump`
  (params (Key :type "Key Structure"))
  (:`Pressed`
    (if (`self.Wallsliding`)
      (`self.Wall Jump`)
      (else
        (`self.Jump`)
        (set `self.JumpMaxCount` 2))))
  (:`Released`
    (`self.StopJumping`)))

(event `Wall Jump`
  (bind (_returnvalue_roll _returnvalue_pitch _returnvalue_yaw) (`KismetMathLibrary.BreakRotator` (`self.K2_GetActorRotation`)))
  (`self.K2_SetActorRotation` (`KismetMathLibrary.MakeRotator` 0.0 0.0 _returnvalue_yaw))
  (`self.LaunchCharacter` (+ (* (`self.GetActorForwardVector`) 300.0) (`KismetMathLibrary.MakeVector` 0.0 0.0 (`CharacterMovementComponent.JumpZVelocity` (`self.CharacterMovement`)))) false true))

(event `InputAxis|right`
  (params (AxisValue :type "Float (single-precision)"))
  (`self.AddMovementInput` (1.0 0.0 0.0) AxisValue))

(event `animation_changer`
  (if (not (`self.Attack`))
    (`PaperFlipbookComponent.SetFlipbook` (`self.Sprite`) (select `bool` (`self.Wallsliding`) :`false` (select `bool` (> (.z (`MovementComponent.Velocity` (`self.CharacterMovement`))) 0.0) :`false` (select `bool` (< (.z (`MovementComponent.Velocity` (`self.CharacterMovement`))) 0.0) :`false` (select `bool` (> (`KismetMathLibrary.VSize` (`MovementComponent.Velocity` (`self.CharacterMovement`))) 0.0) :`false` "/Game/Maps/purple_guy/idle_thicc_legs/idle_animation.idle_animation" :`true` "/Game/Maps/purple_guy/run/run_animation.run_animation" :!type "PaperFlipbook Object Reference") :`true` "/Game/Maps/purple_guy/falling/falling_animation.falling_animation") :`true` "/Game/Maps/purple_guy/jump/jump_animation.jump_animation") :`true` "/Game/Maps/purple_guy/wallslide/wallslide_animation.wallslide_animation"))))

(event `InputAction|attack`
  (params (Key :type "Key Structure"))
  (:`Pressed`
    (`PaperFlipbookComponent.SetFlipbook` (`self.Sprite`) "/Game/Maps/purple_guy/attack/attack_animation.attack_animation")
    (set `self.Attack` true)
    (`KismetSystemLibrary.Delay` 0.2)
    (set `self.Attack` false)))

(event `player_rotation`
  (`/Engine/EditorBlueprintResources/StandardMacros.IsValid` (`self.GetController`)
    (:`Is Valid`
      (`/Engine/EditorBlueprintResources/StandardMacros.CompareFloat` (.x (`MovementComponent.Velocity` (`self.CharacterMovement`)))
        (:`>`
          (`Controller.SetControlRotation` (`self.GetController`) (`KismetMathLibrary.MakeRotator` 0.0)))
        (:`<`
          (`Controller.SetControlRotation` (`self.GetController`) (`KismetMathLibrary.MakeRotator` 0.0 0.0 180.0)))))))

(event `self.ReceiveTick`
  (params (DeltaSeconds :type "Float (single-precision)"))
  (`self.animation_changer`)
  (`self.player_rotation`)
  (`self.Wallslide`))

(fn `UserConstructionScript`)